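; BP_PAWN is a mouse-driven camera pawn that zooms, orbits and pans the view.
; The wheel changes the SpringArm length within min/max limits.
; Holding right mouse rotates the Arrow component's yaw and pitch, with no pitch clamp.
; Otherwise, holding left mouse moves the actor along the Arrow's right and forward vectors, sweeping only on horizontal mouse movement.
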(event `Key|MouseScrollDown`
  (params (Key :type "Key Structure"))
  (bind _returnvalue (+ (`SpringArmComponent.TargetArmLength` (`self.SpringArm`)) (`self.相机缩放速度`)))
  ;[1 1 1] 人物缩放
  ;;[1 1 1] 鼠标下滚控制摄像机视角拉远
  (:`Pressed`
    (if (< _returnvalue (`self.最大目标臂长度`))
      (set `SpringArmComponent.TargetArmLength` _returnvalue (`self.SpringArm`)))))

(event `Key|MouseScrollUp`
  (params (Key :type "Key Structure"))
  (bind _returnvalue (- (`SpringArmComponent.TargetArmLength` (`self.SpringArm`)) (`self.相机缩放速度`)))
  ;[1 1 1] 人物缩放
  ;;[1 1 1] 鼠标上滚控制摄像机视角拉近
  (:`Pressed`
    (if (> _returnvalue (`self.最小目标臂长度`))
      (set `SpringArmComponent.TargetArmLength` _returnvalue (`self.SpringArm`)))))

(event `self.ReceiveBeginPlay`)

(event `Key|LeftMouseButton`
  (params (Key :type "Key Structure"))
  ;[1 1 1] 鼠标左右键分别控制点击变量
  (:`Pressed`
    (set `self.isLeftMouseDown` true))
  (:`Released`
    (set `self.isLeftMouseDown` false)))

(event `InputAxisKey|MouseX`
  (params (AxisValue :type "Float (single-precision)"))
  (bind _arrow (`self.Arrow`))
  (bind (_returnvalue_roll _returnvalue_pitch _returnvalue_yaw) (`KismetMathLibrary.BreakRotator` (`SceneComponent.K2_GetComponentRotation` _arrow)))
  ;[1 1 1] 人物旋转——鼠标X控制世界Z轴旋转（即屏幕左右）并通过左键控制
  (if (`self.isRightMouseDown`)
    (`SceneComponent.K2_SetWorldRotation` _arrow (`KismetMathLibrary.MakeRotator` 0.0 _returnvalue_pitch (+ (* AxisValue (`self.缩放速度`)) _returnvalue_yaw)) false false)
    (else
      ;[1 1 1] 人物（视角中心）屏幕左右位移并通过右键控制
      (if (`self.isLeftMouseDown`)
        (`self.K2_SetActorLocation` (+ (* (* AxisValue (`self.位移速度`)) (`SceneComponent.GetRightVector` (`self.Arrow`))) (`self.K2_GetActorLocation`)) true true)))))

(event `Key|RightMouseButton`
  (params (Key :type "Key Structure"))
  ;[1 1 1] 鼠标左右键分别控制点击变量
  (:`Pressed`
    (set `self.isRightMouseDown` true))
  (:`Released`
    (set `self.isRightMouseDown` false)))

(event `InputAxisKey|MouseY`
  (params (AxisValue :type "Float (single-precision)"))
  (bind _arrow (`self.Arrow`))
  (bind (_returnvalue_roll _returnvalue_pitch _returnvalue_yaw) (`KismetMathLibrary.BreakRotator` (`SceneComponent.K2_GetComponentRotation` _arrow)))
  ;[1 1 1] 人物旋转——鼠标Y控制世界Y轴旋转（即屏幕上下）并通过左键控制
  (if (`self.isRightMouseDown`)
    (`SceneComponent.K2_SetWorldRotation` _arrow (`KismetMathLibrary.MakeRotator` 0.0 (+ (* AxisValue (`self.缩放速度`)) _returnvalue_pitch) _returnvalue_yaw) false false)
    (else
      ;[1 1 1] 人物（视角中心）屏幕上下位移并通过右键控制
      (if (`self.isLeftMouseDown`)
        (`self.K2_SetActorLocation` (+ (`self.K2_GetActorLocation`) (* (* AxisValue (`self.位移速度`)) (`SceneComponent.GetForwardVector` (`self.Arrow`)))))))))

(fn `UserConstructionScript`)